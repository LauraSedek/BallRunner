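; Cannon actor that automatically fires projectiles on a repeating cycle from BeginPlay.
; After a delay set by CannonFireRate, it spawns a BP_Projectile at the Arrow component's location and rotation, scaled by ProjectileScale.
; CannonFireTimeline then animates the barrel along its local Y axis, and its Cannon Fire event track loops back to the delay to keep the cycle running.
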(event EventBeginPlay
  (bind _arrow (Variables|Default|GetArrow))
  (Utilities|FlowControl|Delay (Variables|Cannonproperties|GetCannon%20fire%20rate) :!label _label)
  (Game|SpawnActorfromClass "/Game/Blueprints/Actors/Projectiles/BP_Projectile.BP_Projectile_C" (Math|Transform|MakeTransform (Transformation|GetWorldLocation _arrow) (Transformation|GetWorldRotation _arrow) (Math|Conversions|ToVector(Float) (Variables|CannonProperties|GetProjectile%20scale))) "Undefined" 0 0)
  (bind _cannon_barrel_location (Timeline|Cannon%20fire%20timeline PlayFromStart)
    (:Update
      (Transformation|SetRelativeLocation (Variables|Default|GetCannon) (Math|Vector|MakeVector 0.0 _cannon_barrel_location 0.0) false false))
    (:Cannon%20fire
      (goto _label))))

(fn ConstructionScript)