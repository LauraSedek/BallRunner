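; Player pawn for a physics-driven sphere that the player moves with left/right and forward/backward axis input.
; Both axes apply torque to the Sphere as acceleration change, scaled by MagicNumber.
; BeginPlay fades the camera in, and any damage triggers the Restart level macro.
; That macro runs once, fading the camera out and reopening the current level by name after a short delay.
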(event EventBeginPlay
  (CameraFades|StartCameraFade :self (Game|GetPlayerCameraManager 0) :FromAlpha 1.0 :Duration 3.0))

(event Game|Damage|EventAnyDamage
  (params (Damage :type Float%20%28single-precision%29) (DamageType :type Damage%20Type%20Object%20Reference) (InstigatedBy :type Controller%20Object%20Reference) (DamageCauser :type Actor%20Object%20Reference))
  (Utilities|RestartLevel))

(event Input|AxisEvents|InputAxisMoveForward/Backward
  (params (AxisValue :type Float%20%28single-precision%29))
  (Class|PrimitiveComponent|AddTorqueinRadians (Variables|Default|GetSphere) (Math|Vector|MakeVector (* (stale Input|AxisEvents|InputAxisMoveLeft/Right AxisValue) (Variables|Default|GetMagicNumber)) (* AxisValue (Variables|Default|GetMagicNumber)) 0.0) "None" true))

(event Input|AxisEvents|InputAxisMoveLeft/Right
  (params (AxisValue :type Float%20%28single-precision%29))
  (Class|PrimitiveComponent|AddTorqueinRadians (Variables|Default|GetSphere) (Math|Vector|MakeVector (* AxisValue (Variables|Default|GetMagicNumber)) (* (stale Input|AxisEvents|InputAxisMoveForward/Backward AxisValue) (Variables|Default|GetMagicNumber)) 0.0) "None" true))

(fn ConstructionScript)